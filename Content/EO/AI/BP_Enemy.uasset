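; Enemy AI that, once Pawn Sensing sees a pawn, chases the player and takes up a position around them.
; AI MoveTo is reissued every tick to close in, returning any held slot to BP_Manager's shared offset array.
; On success it claims the nearest player-relative slot by removing it from that array.
; It then faces the player, moves there by setting its location, snapping and rotating Cube1 on arrival.
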(event OnSeePawn(PawnSensing)
  (params (Pawn :type Pawn%20Object%20Reference))
  (Variables|Default|SetIsSeeing true))

(event EventBeginPlay)

(event EventTick
  (params (DeltaSeconds :type Float%20%28single-precision%29))
  (Variables|Default|SetDeltaSecond DeltaSeconds)
  (if (not (Variables|Default|GetIsDead))
    (if (Variables|Default|GetIsSeeing)
      (AI|AIMoveTo self "0, 0, 0" (Game|GetPlayerCharacter 0) 8e+02 false
        (:then
          (if (not (Class|KismetMathLibrary|EqualExactlyVectorVector (Variables|Default|GetAroundPosVector) "0, 0, 0"))
            (Utilities|Array|Add (Variables|/Game/EO/AI/BP_Manager.BP_Manager_C|GetArrVector (Variables|Default|GetBP_Manager)) (Variables|Default|GetUsedVector))
            (Variables|Default|SetAroundPosVector "0, 0, 0")))
        (:OnSuccess
          (CallFunction|GetAroundPosition)
          (Transformation|SetActorRotation (Math|Rotator|FindLookatRotation (Transformation|GetActorLocation) (Transformation|GetActorLocation (Game|GetPlayerCharacter 0))))
          (CallFunction|ActorMoveto (Variables|Default|GetAroundPosVector) 3e+02)
          (if (>= 3.0 (Math|Vector|Distance(Vector) (Variables|Default|GetAroundPosVector) (Transformation|GetActorLocation)))
            (Transformation|SetActorLocation (Variables|Default|GetAroundPosVector) false false)
            (Transformation|AddLocalRotation (Variables|Default|GetCube1) "0.000000,0.000000,10.000000" false false)))))))

(fn ConstructionScript)

(fn ActorMoveto
  (params (Direction :type Vector) (Speed :type Float%20%28double-precision%29))
  (Transformation|SetActorLocation (+ (Transformation|GetActorLocation) (* (Variables|Default|GetDeltaSecond) (* (Math|Vector|Normalize (- Direction (Transformation|GetActorLocation))) Speed))) false false))

(fn GetAroundPosition
  (bind _returnvalue (Actor|GetActorOfClass "/Game/EO/AI/BP_Manager.BP_Manager_C"))
  (bind _output_get (Variables|Default|SetBP_Manager _returnvalue))
  (Variables|Default|Setmin 1e+03)
  (for (_array_element _array_index) (Variables|/Game/EO/AI/BP_Manager.BP_Manager_C|GetArrVector _output_get)
    (if (> (Variables|Default|Getmin) (Math|Vector|Distance(Vector) (+ _array_element (Transformation|GetActorLocation (Game|GetPlayerCharacter 0))) (Transformation|GetActorLocation)))
      (Variables|Default|Setmin (Math|Vector|Distance(Vector) (+ _array_element (Transformation|GetActorLocation (Game|GetPlayerCharacter 0))) (Transformation|GetActorLocation)))
      (Variables|Default|SetArrIndex _array_index)))
  (bind _output_get_2 (Variables|Default|SetUsedVector (Utilities|Array|Get(acopy) (Variables|/Game/EO/AI/BP_Manager.BP_Manager_C|GetArrVector (Variables|Default|GetBP_Manager)) (Variables|Default|GetArrIndex))))
  (if (Class|KismetMathLibrary|EqualExactlyVectorVector (Variables|Default|GetAroundPosVector) "0, 0, 0")
    (Variables|Default|SetAroundPosVector (+ _output_get_2 (Transformation|GetActorLocation (Game|GetPlayerCharacter 0))))
    (Utilities|Array|RemoveItem (Variables|/Game/EO/AI/BP_Manager.BP_Manager_C|GetArrVector (Variables|Default|GetBP_Manager)) (Variables|Default|GetUsedVector))))