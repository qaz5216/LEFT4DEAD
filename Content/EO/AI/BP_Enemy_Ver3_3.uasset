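; Enemy AI character that chases the first player once pawn sensing spots a pawn and takes damage from FPS projectiles.
; Tick drives AIMoveTo and updates CanAttack by distance after the move request is issued; IsSeeing is never cleared.
; Head, body and leg overlaps apply descending damage, while PlayerAttack removes player HP.
; At zero HP, Tick stops movement, disables collision and destroys the actor after a delay.
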(event OnSeePawn(PawnSensing)
  (params (Pawn :type Pawn%20Object%20Reference))
  (Variables|Default|SetIsSeeing true))

(event OnComponentBeginOverlap(Head)
  (params (OverlappedComponent :type Primitive%20Component%20Object%20Reference) (OtherActor :type Actor%20Object%20Reference) (OtherComp :type Primitive%20Component%20Object%20Reference) (OtherBodyIndex :type Integer) (bFromSweep :type Boolean) (SweepResult :type Hit%20Result%20Structure%20%28by%20ref%29))
  (Utilities|Casting|CastToBP_FPSProjectile OtherActor)
  (Variables|Default|SetIsHit true)
  (bind _output_get (Variables|Default|SetDamage 8))
  (CallFunction|TakeDamage _output_get))

(event OnComponentBeginOverlap(Body)
  (params (OverlappedComponent :type Primitive%20Component%20Object%20Reference) (OtherActor :type Actor%20Object%20Reference) (OtherComp :type Primitive%20Component%20Object%20Reference) (OtherBodyIndex :type Integer) (bFromSweep :type Boolean) (SweepResult :type Hit%20Result%20Structure%20%28by%20ref%29))
  (Utilities|Casting|CastToBP_FPSProjectile OtherActor)
  (Variables|Default|SetIsHit true)
  (bind _output_get (Variables|Default|SetDamage 2))
  (CallFunction|TakeDamage _output_get))

(event OnComponentBeginOverlap(Leg)
  (params (OverlappedComponent :type Primitive%20Component%20Object%20Reference) (OtherActor :type Actor%20Object%20Reference) (OtherComp :type Primitive%20Component%20Object%20Reference) (OtherBodyIndex :type Integer) (bFromSweep :type Boolean) (SweepResult :type Hit%20Result%20Structure%20%28by%20ref%29))
  (Utilities|Casting|CastToBP_FPSProjectile OtherActor)
  (Variables|Default|SetIsHit true)
  (bind _output_get (Variables|Default|SetDamage 1))
  (CallFunction|TakeDamage _output_get))

(event Custom|PlayerAttack
  (bind _asbp_fpscharacter (Utilities|Casting|CastToBP_FPSCharacter (Game|GetPlayerCharacter 0)))
  (Variables|/Script/ProjectMove.FPSCharacter|SetHP _asbp_fpscharacter (- (Variables|/Script/ProjectMove.FPSCharacter|GetHP _asbp_fpscharacter) 1)))

(event EventTick
  (params (DeltaSeconds :type Float%20%28single-precision%29))
  (if (Variables|Default|GetIsDead)
    (Variables|/Script/Engine.CharacterMovementComponent|SetMaxWalkSpeed (Variables|Character|GetCharacterMovement) 0.0)
    (CallFunction|DisableCollision)
    (Utilities|FlowControl|Delay 5.0)
    (Actor|DestroyActor)
    (elif (Variables|Default|GetIsSeeing)
      (AI|AIMoveTo self "0, 0, 0" (Game|GetPlayerCharacter 0) 6e+01 false
        (:then
          (if (<= (Math|Vector|Distance(Vector) (Transformation|GetActorLocation (Game|GetPlayerCharacter 0)) (Transformation|GetActorLocation)) 75.0)
            (Variables|Default|SetCanAttack true)
            (else
              (Variables|Default|SetCanAttack false))))))))

(fn ConstructionScript)

(fn TakeDamage
  (params (Damage :type Integer))
  (bind _output_get (Variables|Default|SetHP (- (Variables|Default|GetHP) Damage)))
  (if (<= _output_get 0)
    (Variables|Default|SetIsDead true)))

(fn DisableCollision
  (Collision|SetCollisionEnabled (Variables|Collision|GetCapsuleComponent) "NoCollision")
  (Collision|SetCollisionEnabled (Variables|Default|GetHead) "NoCollision")
  (Collision|SetCollisionEnabled (Variables|Default|GetLeg) "NoCollision")
  (Collision|SetCollisionEnabled (Variables|Default|GetBody) "NoCollision"))