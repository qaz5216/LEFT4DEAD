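; AI manager Blueprint that precomputes a ring of offset vectors, named as positions around the player.
; On BeginPlay, SetAroundPlayerPosition steps yaw by 360 / Count to build 16 flat directions scaled to 200 units and appends them to ArrVector.
; The vectors are origin-relative: the graph never reads the player's location or uses the array, and Tick and overlap events are empty.
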(event EventBeginPlay
  (CallFunction|SetAroundPlayerPosition 2e+02 16))

(event Collision|EventActorBeginOverlap
  (params (OtherActor :type Actor%20Object%20Reference)))

(event EventTick
  (params (DeltaSeconds :type Float%20%28single-precision%29)))

(fn ConstructionScript)

(fn SetAroundPlayerPosition
  (params (Distance :type Float%20%28double-precision%29) (Count :type Integer))
  (for _index (range 1 Count)
    (Utilities|Array|Add (Variables|Default|GetArrVector) (* Distance (Math|Vector|Normalize (Class|KismetMathLibrary|CreateVectorfromYawPitch (* (/ (Variables|Default|Get360) Count) _index) 0.0 1.0))))))