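; Enemy that, once it sees the player, surrounds and attacks them, and dies after enough projectile hits.
; Each tick it claims the nearest free player-relative offset from BP_Manager's shared array, returning it while still travelling and keeping it on arrival.
; Movement is manual location and rotation updates.
; At its slot it rotates Cube1 and damages the player after a delay, moving again if the player leaves range.
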(event OnSeePawn(PawnSensing)
  (params (Pawn :type Pawn%20Object%20Reference))
  (Variables|Default|SetIsSeeing true))

(event OnComponentBeginOverlap(CapsuleComponent)
  (params (OverlappedComponent :type Primitive%20Component%20Object%20Reference) (OtherActor :type Actor%20Object%20Reference) (OtherComp :type Primitive%20Component%20Object%20Reference) (OtherBodyIndex :type Integer) (bFromSweep :type Boolean) (SweepResult :type Hit%20Result%20Structure%20%28by%20ref%29))
  (Utilities|Casting|CastToBP_FPSProjectile OtherActor)
  (bind _output_get (Variables|Default|SetHP (- (Variables|Default|GetHP) 1)))
  (if (<= _output_get 0)
    (Variables|Default|SetIsDead true)))

(event EventBeginPlay
  (bind _returnvalue (Actor|GetActorOfClass "/Game/EO/AI/BP_Manager.BP_Manager_C"))
  (Variables|Default|SetBP_Manager _returnvalue))

(event EventTick
  (params (DeltaSeconds :type Float%20%28single-precision%29))
  (bind _returnvalue (Transformation|GetActorLocation))
  (bind _returnvalue_2 (Game|GetPlayerCharacter 0))
  (bind _returnvalue_3 (Transformation|GetActorLocation _returnvalue_2))
  (Variables|Default|SetDeltaSecond DeltaSeconds)
  (if (Variables|Default|GetIsDead)
    (Actor|DestroyActor)
    (elif (Variables|Default|GetIsSeeing)
      (CallFunction|GetAroundPosition)
      (if (Variables|Default|GetCanMove)
        (CallFunction|ActorMoveto (Variables|Default|GetAroundPosVector) 3e+02)
        (Transformation|SetActorRotation (Math|Rotator|FindLookatRotation (Math|Vector|MakeVector (.x _returnvalue) (.y _returnvalue) 0.0) (Math|Vector|MakeVector (.x _returnvalue_3) (.y _returnvalue_3) 0.0)))
        (if (>= 3.0 (Math|Vector|Distance(Vector) (Variables|Default|GetAroundPosVector) (Transformation|GetActorLocation)))
          (Variables|Default|SetCanMove false)
          (elif (Variables|Default|GetIsRemoved)
            (Utilities|Array|Add (Variables|/Game/EO/AI/BP_Manager.BP_Manager_C|GetArrVector (Variables|Default|GetBP_Manager)) (Variables|Default|GetUsedVector))
            (Variables|Default|SetIsRemoved false)))
        (elif (<= (Math|Vector|Distance(Vector) (Transformation|GetActorLocation (Game|GetPlayerCharacter 0)) (Transformation|GetActorLocation)) 2.1e+02)
          (Transformation|AddLocalRotation (Variables|Default|GetCube1) "0.000000,0.000000,10.000000" false false)
          (Utilities|FlowControl|Delay 2.0)
          (bind _asbp_fpscharacter (Utilities|Casting|CastToBP_FPSCharacter (Game|GetPlayerCharacter 0)))
          (Class|FPSCharacter|Attacked _asbp_fpscharacter 10)
          (else
            (Variables|Default|SetCanMove true)))))))

(fn ConstructionScript)

(fn ActorMoveto
  (params (Direction :type Vector) (Speed :type Float%20%28double-precision%29))
  (Transformation|SetActorLocation (+ (Transformation|GetActorLocation) (* (Variables|Default|GetDeltaSecond) (* (Math|Vector|Normalize (- Direction (Transformation|GetActorLocation))) Speed))) false false))

(fn GetAroundPosition
  (Variables|Default|Setmin 1e+03)
  (for (_array_element _array_index) (Variables|/Game/EO/AI/BP_Manager.BP_Manager_C|GetArrVector (Variables|Default|GetBP_Manager))
    (if (> (Variables|Default|Getmin) (Math|Vector|Distance(Vector) (+ _array_element (Transformation|GetActorLocation (Game|GetPlayerCharacter 0))) (Transformation|GetActorLocation)))
      (Variables|Default|Setmin (Math|Vector|Distance(Vector) (+ _array_element (Transformation|GetActorLocation (Game|GetPlayerCharacter 0))) (Transformation|GetActorLocation)))
      (Variables|Default|SetArrIndex _array_index)))
  (if (Variables|Default|GetIsRemoved)
    (Variables|Default|SetAroundPosVector (+ (Variables|Default|GetUsedVector) (Transformation|GetActorLocation (Game|GetPlayerCharacter 0))))
    (else
      (bind _output_get (Variables|Default|SetUsedVector (Utilities|Array|Get(acopy) (Variables|/Game/EO/AI/BP_Manager.BP_Manager_C|GetArrVector (Variables|Default|GetBP_Manager)) (Variables|Default|GetArrIndex))))
      (Variables|Default|SetAroundPosVector (+ _output_get (Transformation|GetActorLocation (Game|GetPlayerCharacter 0))))
      (Utilities|Array|RemoveIndex (Variables|/Game/EO/AI/BP_Manager.BP_Manager_C|GetArrVector (Variables|Default|GetBP_Manager)) (Variables|Default|GetArrIndex))
      (Variables|Default|SetIsRemoved true))))