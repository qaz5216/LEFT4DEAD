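; BP_ElevatorLDoor is an elevator door actor, likely the left one, that slides while the elevator controller reports a press.
; On BeginPlay it finds and caches the BP_ElevatorController in the level.
; Each Tick, while Ispress is true, it moves along a forward vector scaled by Speed and delta time.
; It snaps to and stops at the world origin once within one unit of it.
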(event EventBeginPlay
  (bind _returnvalue (Actor|GetActorOfClass "/Game/EO/Blueprints/BP_ElevatorController.BP_ElevatorController_C"))
  (Variables|Default|SetElevatorController _returnvalue))

(event Collision|EventActorBeginOverlap
  (params (OtherActor :type Actor%20Object%20Reference)))

(event EventTick
  (params (DeltaSeconds :type Float%20%28single-precision%29))
  (Variables|Default|SetDeltaTime DeltaSeconds)
  (if (and (Variables|/Script/ProjectMove.Elevator|Getispress (Variables|Default|GetElevatorController)) (Class|KismetMathLibrary|NotEqualExactlyVectorVector (Transformation|GetActorLocation) "0, 0, 0"))
    (Transformation|SetActorLocation (+ (Transformation|GetActorLocation) (* (* (Class|KismetMathLibrary|VectorForward) (Variables|Default|GetSpeed)) (Variables|Default|GetDeltaTime))) false false)
    (if (not (>= (Math|Vector|Distance(Vector) (Transformation|GetActorLocation) "0, 0, 0") 1.0))
      (Transformation|SetActorLocation "0, 0, 0" false false))))

(fn ConstructionScript)